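; BP_Block is a placeable block for the builder that can be nudged along each axis and highlighted when selected.
; Six move functions shift the static mesh by half its height, depth or width, then snap the location to a fixed grid.
; Selected and Deselected swap the mesh's overlay material, and BeginPlay marks a new block as selected.
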(event `self.ReceiveBeginPlay`
  (`self.Selected`))

(fn `Deselected`
  (`MeshComponent.SetOverlayMaterial` (`self.StaticMesh`) "/Game/Builder/Materials/MI_Overlay_Deselected.MI_Overlay_Deselected"))

(fn `Move Block Downwards`
  (bind _staticmesh (`self.StaticMesh`))
  (`SceneComponent.K2_SetWorldLocation` _staticmesh (`KismetMathLibrary.Vector_SnappedToGrid` (- (`SceneComponent.K2_GetComponentLocation` _staticmesh) (`KismetMathLibrary.MakeVector` 0.0 0.0 (/ (`self.Mesh Height`) 2.0))) 50.0) false false))

(fn `Move Block Upwards`
  (bind _staticmesh (`self.StaticMesh`))
  (`SceneComponent.K2_SetWorldLocation` _staticmesh (`KismetMathLibrary.Vector_SnappedToGrid` (+ (`SceneComponent.K2_GetComponentLocation` _staticmesh) (`KismetMathLibrary.MakeVector` 0.0 0.0 (/ (`self.Mesh Height`) 2.0))) 50.0) false false))

(fn `Move Block X Negative`
  (bind _staticmesh (`self.StaticMesh`))
  (`SceneComponent.K2_SetWorldLocation` _staticmesh (`KismetMathLibrary.Vector_SnappedToGrid` (- (`SceneComponent.K2_GetComponentLocation` _staticmesh) (`KismetMathLibrary.MakeVector` (/ (`self.Mesh Depth`) 2.0))) 50.0) false false))

(fn `Move Block X Positive`
  (bind _staticmesh (`self.StaticMesh`))
  (`SceneComponent.K2_SetWorldLocation` _staticmesh (`KismetMathLibrary.Vector_SnappedToGrid` (+ (`SceneComponent.K2_GetComponentLocation` _staticmesh) (`KismetMathLibrary.MakeVector` (/ (`self.Mesh Depth`) 2.0))) 50.0) false false))

(fn `Move Block Y Negative`
  (bind _staticmesh (`self.StaticMesh`))
  (`SceneComponent.K2_SetWorldLocation` _staticmesh (`KismetMathLibrary.Vector_SnappedToGrid` (- (`SceneComponent.K2_GetComponentLocation` _staticmesh) (`KismetMathLibrary.MakeVector` 0.0 (/ (`self.Mesh Width`) 2.0))) 50.0) false false))

(fn `Move Block Y Positive`
  (bind _staticmesh (`self.StaticMesh`))
  (`SceneComponent.K2_SetWorldLocation` _staticmesh (`KismetMathLibrary.Vector_SnappedToGrid` (+ (`SceneComponent.K2_GetComponentLocation` _staticmesh) (`KismetMathLibrary.MakeVector` 0.0 (/ (`self.Mesh Width`) 2.0))) 50.0) false false))

(fn `Selected`
  (`MeshComponent.SetOverlayMaterial` (`self.StaticMesh`) "/Game/Builder/Materials/MI_Overlay_Selected.MI_Overlay_Selected"))

(fn `UserConstructionScript`)