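; Player pawn for a block-building mode that places, selects and nudges BP_Block actors with mouse and keyboard.
; Left click traces from the cursor: a block hit selects it and sets the build spot off the hit face, while other hits clear selection and snap the spot to a grid.
; F spawns and selects a block there.
; Keys move the current block along three axes, with a tracked array keeping selection exclusive.
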(event `Key|LeftMouseButton`
  (params (Key :type "Key Structure"))
  ;[1 1 1] Select Location
  (:`Pressed`
    (`self.Select Location`)))

(event `Key|F`
  (params (Key :type "Key Structure"))
  ;[1 1 1] Create Mesh
  (:`Pressed`
    (`self.Create Block` "/Game/Builder/Blueprints/BP_Block.BP_Block_C")))

(event `Key|U`
  (params (Key :type "Key Structure"))
  ;[1 1 1] Up and Down
  (:`Pressed`
    (`/Game/Builder/Blueprints/BP_Block.Move Block Upwards` (`self.Current Block`))))

(event `Key|J`
  (params (Key :type "Key Structure"))
  ;[1 1 1] Up and Down
  (:`Pressed`
    (`/Game/Builder/Blueprints/BP_Block.Move Block Downwards` (`self.Current Block`))))

(event `Key|K`
  (params (Key :type "Key Structure"))
  ;[1 1 1] X positive and negative
  (:`Pressed`
    (`/Game/Builder/Blueprints/BP_Block.Move Block X Positive` (`self.Current Block`))))

(event `Key|H`
  (params (Key :type "Key Structure"))
  ;[1 1 1] X positive and negative
  (:`Pressed`
    (`/Game/Builder/Blueprints/BP_Block.Move Block X Negative` (`self.Current Block`))))

(event `Key|Y`
  (params (Key :type "Key Structure"))
  ;[1 1 1] Y positive and negative
  (:`Pressed`
    (`/Game/Builder/Blueprints/BP_Block.Move Block Y Positive` (`self.Current Block`))))

(event `Key|I`
  (params (Key :type "Key Structure"))
  ;[1 1 1] Y positive and negative
  (:`Pressed`
    (`/Game/Builder/Blueprints/BP_Block.Move Block Y Negative` (`self.Current Block`))))

(fn `Clear Blocks Selection`
  (for _array_element (`self.Blocks`)
    (`/Game/Builder/Blueprints/BP_Block.Deselected` _array_element)
    (set `self.Current Block` null)))

(fn `Create Block`
  (params (NewParam :type "/Game/Builder/Blueprints/BP_Block Class Reference"))
  (bind _returnvalue (`|SpawnActorFromClass` NewParam (`self.Build Location`) "AdjustIfPossibleButAlwaysSpawn" "MultiplyWithRoot" null null))
  (`KismetArrayLibrary.Array_AddUnique` (`self.Blocks`) _returnvalue)
  (`self.Select Block` _returnvalue))

(fn `Select Block`
  (params (`Current Block` :type "/Game/Builder/Blueprints/BP_Block Object Reference"))
  (`self.Clear Blocks Selection`)
  (bind _output_get (set `self.Current Block` `Current Block`))
  (`/Game/Builder/Blueprints/BP_Block.Selected` _output_get))

(fn `Select Location`
  (bind (_worldlocation _worlddirection) (`PlayerController.DeprojectMousePositionToWorld` (`GameplayStatics.GetPlayerController` 0)))
  (bind (_outhit _returnvalue) (`KismetSystemLibrary.LineTraceSingle` :`Start` _worldlocation :`End` (+ _worldlocation (* _worlddirection 12000)) :`TraceChannel` "TraceTypeQuery1" :`DrawDebugType` "ForDuration"))
  (if _returnvalue
    (bind (_bblockinghit _binitialoverlap _time _distance _location _impactpoint _normal _impactnormal _physmat _hitactor) (`GameplayStatics.BreakHitResult` _outhit))
    (bind _asbp_block (cast `/Game/Builder/Blueprints/BP_Block` _hitactor)
      (:`then`
        (`self.Select Block` _asbp_block)
        (set `self.Build Location` (`KismetMathLibrary.MakeTransform` (+ _location (* _normal (50.0 50.0 50.0))))))
      (:`CastFailed`
        (`self.Clear Blocks Selection`)
        (set `self.Build Location` (`KismetMathLibrary.MakeTransform` (`KismetMathLibrary.Vector_SnappedToGrid` (+ _location (0.0 0.0 50.0)) 50.0)))))))

(fn `UserConstructionScript`)